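; Game mode for a root-growing game that shows the main menu on BeginPlay and starts the player's BP_CurrentRoot pawn on LaunchGame.
; Bonus and malus events set the pawn's turn rate or root time, then restore fixed values after a Delay.
; IncreaseMiningSpeed writes the same value before and after its delay, while StopStamina and Sway are empty.
; MakeRootFragile decrements LifePoint, calling BreakRoot at zero to halt mining.
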(event Custom|LaunchGame
  (Default|Play (.AsBP%20Current%20Root (Utilities|Casting|CastToBP_CurrentRoot (Game|Player|GetPlayerPawn 0)))))

(event EventBeginPlay
  (bind _returnvalue (UserInterface|CreateWidget "/Game/Sasha/W_MainMenu.W_MainMenu_C"))
  (UserInterface|Viewport|AddtoViewport _returnvalue 0))

(event EventStopStamina)

(event EventIncreaseSoftness
  (bind _returnvalue (Game|Player|GetPlayerPawn 0))
  (bind _asbp_current_root (Utilities|Casting|CastToBP_CurrentRoot _returnvalue))
  (Variables|/Game/Blueprints/BP_CurrentRoot.BP_CurrentRoot_C|SetTurnRate _asbp_current_root 2.0)
  (Utilities|FlowControl|Delay 3.0)
  (Variables|/Game/Blueprints/BP_CurrentRoot.BP_CurrentRoot_C|SetTurnRate _asbp_current_root 1.0))

(event EventIncreaseDurability
  (bind _returnvalue (Game|Player|GetPlayerPawn 0))
  (bind _asbp_current_root (Utilities|Casting|CastToBP_CurrentRoot _returnvalue))
  (Variables|/Game/Blueprints/BP_CurrentRoot.BP_CurrentRoot_C|SetTimeForRoot _asbp_current_root 2e+01)
  (Utilities|FlowControl|Delay 3.0)
  (Variables|/Game/Blueprints/BP_CurrentRoot.BP_CurrentRoot_C|SetTimeForRoot _asbp_current_root 15.0))

(event EventIncreaseMiningSpeed
  (bind _returnvalue (Game|Player|GetPlayerPawn 0))
  (bind _asbp_current_root (Utilities|Casting|CastToBP_CurrentRoot _returnvalue))
  (Variables|/Game/Blueprints/BP_CurrentRoot.BP_CurrentRoot_C|SetMiningSpeed _asbp_current_root 1.2)
  (Utilities|FlowControl|Delay 2.0)
  (Variables|/Game/Blueprints/BP_CurrentRoot.BP_CurrentRoot_C|SetMiningSpeed _asbp_current_root 1.2))

(event EventSway)

(event EventMakeRootFragile
  (bind _result (Math|Integer|DecrementInt (Variables|Default|GetLifePoint))
    (:%20%20
      (if (not (> _result 0))
        (Class|InteractibleInterface|BreakRoot)))))

(event EventDecreaseSoftness
  (bind _returnvalue (Game|Player|GetPlayerPawn 0))
  (bind _asbp_current_root (Utilities|Casting|CastToBP_CurrentRoot _returnvalue))
  (Variables|/Game/Blueprints/BP_CurrentRoot.BP_CurrentRoot_C|SetTurnRate _asbp_current_root 0.5)
  (Utilities|FlowControl|Delay 3.0)
  (Variables|/Game/Blueprints/BP_CurrentRoot.BP_CurrentRoot_C|SetTurnRate _asbp_current_root 1.0))

(event EventBreakRoot
  (Variables|/Game/Blueprints/BP_CurrentRoot.BP_CurrentRoot_C|SetMiningSpeed (.AsBP%20Current%20Root (Utilities|Casting|CastToBP_CurrentRoot (Game|Player|GetPlayerPawn 0))) 0.0))

(fn ConstructionScript)