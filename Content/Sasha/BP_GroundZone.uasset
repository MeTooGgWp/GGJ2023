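; BP_GroundZone is an indexed ground zone that seeds random pickups and sets how fast the root digs inside it.
; The construction script maps the zone Index to bonus and malus count ranges, with higher indices leaning toward fewer bonuses and more maluses.
; BeginPlay spawns random classes from both lists at random points in the Box.
; Overlapping the Box sets BP_CurrentRoot's MiningSpeed, slower for higher indices.
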(event OnComponentBeginOverlap(Box)
  (params (OverlappedComponent :type Primitive%20Component%20Object%20Reference) (OtherActor :type Actor%20Object%20Reference) (OtherComp :type Primitive%20Component%20Object%20Reference) (OtherBodyIndex :type Integer) (bFromSweep :type Boolean) (SweepResult :type Hit%20Result%20Structure%20%28by%20ref%29))
  (bind (_asbp_current_root _bsuccess) (Utilities|Casting|CastToBP_CurrentRoot OtherActor))
  ;[1 1 1] digging difficulty by zone
  (if _bsuccess
    (switch int (Variables|Default|GetIndex)
      (:0
        (Variables|/Game/Blueprints/BP_CurrentRoot.BP_CurrentRoot_C|SetMiningSpeed _asbp_current_root 1.0))
      (:1
        (Variables|/Game/Blueprints/BP_CurrentRoot.BP_CurrentRoot_C|SetMiningSpeed _asbp_current_root 0.8))
      (:2
        (Variables|/Game/Blueprints/BP_CurrentRoot.BP_CurrentRoot_C|SetMiningSpeed _asbp_current_root 0.6))
      (:3
        (Variables|/Game/Blueprints/BP_CurrentRoot.BP_CurrentRoot_C|SetMiningSpeed _asbp_current_root 0.4)))))

(event Custom|SpawnBonuses
  (bind _box (Variables|Default|GetBox))
  (bind _bonuses (Variables|Default|GetBonuses))
  (bind _returnvalue (Transformation|GetWorldLocation _box))
  (bind _boxextent (Variables|/Script/Engine.BoxComponent|GetBoxExtent _box))
  (bind (_x _y) (Math|Vector|BreakVector _boxextent))
  (bind (_x_2 _y_2) (Math|Vector|BreakVector _returnvalue))
  ;[1 1 1] Spawn bonus/malus at the beginning of the game
  (for _index (range 0 (Math|Random|RandomIntegerinRange (Variables|Default|GetMinBonuses) (Variables|Default|GetMaxBonuses)))
    (Game|SpawnActorfromClass (Utilities|Array|Get(acopy) _bonuses (Math|Random|RandomIntegerinRange 0 (- (Utilities|Array|Length _bonuses) 1))) (Math|Transform|MakeTransform (Math|Random|RandomPointinBoundingBox (Math|Vector|MakeVector _x_2 _y_2 7e+01) (Math|Vector|MakeVector _x _y 7e+01))) "Undefined" 0 0)))

(event Custom|SpawnMaluses
  (bind _box (Variables|Default|GetBox))
  (bind _maluses (Variables|Default|GetMaluses))
  (bind _returnvalue (Transformation|GetWorldLocation _box))
  (bind _boxextent (Variables|/Script/Engine.BoxComponent|GetBoxExtent _box))
  (bind (_x _y) (Math|Vector|BreakVector _returnvalue))
  (bind (_x_2 _y_2) (Math|Vector|BreakVector _boxextent))
  ;[1 1 1] Spawn bonus/malus at the beginning of the game
  (for _index (range 0 (Math|Random|RandomIntegerinRange (Variables|Default|GetMinMaluses) (Variables|Default|GetMaxMaluses)))
    (Game|SpawnActorfromClass (Utilities|Array|Get(acopy) _maluses (Math|Random|RandomIntegerinRange 0 (- (Utilities|Array|Length _maluses) 1))) (Math|Transform|MakeTransform (Math|Random|RandomPointinBoundingBox (Math|Vector|MakeVector _x _y 7e+01) (Math|Vector|MakeVector _x_2 _y_2 7e+01))) "Undefined" 0 0)))

(event EventBeginPlay
  (CallFunction|SpawnBonuses)
  (CallFunction|SpawnMaluses))

(fn ConstructionScript
  (switch int (Variables|Default|GetIndex)
    (:0
      (Variables|Default|SetMinBonuses 3)
      (Variables|Default|SetMaxBonuses 4)
      (Variables|Default|SetMinMaluses 0)
      (Variables|Default|SetMaxMaluses 1))
    (:1
      (Variables|Default|SetMinBonuses 2)
      (Variables|Default|SetMaxBonuses 4)
      (Variables|Default|SetMinMaluses 0)
      (Variables|Default|SetMaxMaluses 2))
    (:2
      (Variables|Default|SetMinBonuses 1)
      (Variables|Default|SetMaxBonuses 3)
      (Variables|Default|SetMinMaluses 1)
      (Variables|Default|SetMaxMaluses 2))
    (:3
      (Variables|Default|SetMinBonuses 1)
      (Variables|Default|SetMaxBonuses 2)
      (Variables|Default|SetMinMaluses 2)
      (Variables|Default|SetMaxMaluses 2))))