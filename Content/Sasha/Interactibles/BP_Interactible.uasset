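; BP_Interactible is an interactible that carries a Points value and shows it on a text component.
; The construction script writes Points into the text and colors it green when positive or red when negative.
; AddPoints makes the text visible and returns Points to the caller.
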(fn ConstructionScript
  (bind _textrender (Variables|Default|GetTextRender))
  (bind _points (Variables|Default|GetPoints))
  (Rendering|Components|TextRender|SetText _textrender (Utilities|Text|ToText(Integer) (Variables|Default|GetPoints)))
  (if (> _points 0)
    (Rendering|Components|TextRender|SetTextRenderColor _textrender (Math|Color|MakeColor 0 255 0 255))
    (elif (< _points 0)
      (Rendering|Components|TextRender|SetTextRenderColor _textrender (Math|Color|MakeColor 0 0 255 255)))))

(fn AddPoints
  (Rendering|SetVisibility (Variables|Default|GetTextRender) true false)
  (return (Variables|Default|GetPoints)))