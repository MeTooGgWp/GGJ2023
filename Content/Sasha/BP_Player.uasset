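; Player character that looks around, moves and digs into voxel terrain.
; Axis inputs drive controller pitch and yaw, while Z and E both apply a large forward movement input on each press.
; Dig line-traces along the mesh's forward vector with debug drawing, carving a sphere from the VoxelWorld at the impact point.
; Other hit actors that cast to Interactible receive the hit through OnHitComponent.
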(event Input|ActionEvents|InputActionDig
  (params (Key :type Key%20Structure :default "None"))
  (bind _mesh (Variables|Character|GetMesh))
  (bind _returnvalue (Transformation|GetWorldLocation _mesh))
  (:Pressed
    (bind (_outhit _returnvalue_2) (Collision|LineTraceByChannel _returnvalue (+ _returnvalue (* (Math|Vector|GetForwardVector _mesh) (Variables|Default|GetNewVar_0))) "TraceTypeQuery1" false 0 "ForDuration"))
    (if _returnvalue_2
      (bind _returnvalue_3 (Actor|GetActorOfClass "/Script/Voxel.VoxelWorld"))
      (if (== _returnvalue_3 (.HitActor (Collision|BreakHitResult _outhit)))
        (Class|VoxelSphereTools|RemoveSphere _returnvalue_3 (.ImpactPoint (Collision|BreakHitResult _outhit)) 2.5e+02)
        (elif (.bSuccess (Utilities|Casting|CastToInteractible (.HitActor (Collision|BreakHitResult _outhit))))
          (Class|Interactible|OnHitComponent (.AsInteractible (Utilities|Casting|CastToInteractible (.HitActor (Collision|BreakHitResult _outhit)))) 0 0 0 "0, 0, 0" _outhit))))))

(event Input|AxisEvents|InputAxislookup
  (params (AxisValue :type Float%20%28single-precision%29))
  (Pawn|Input|AddControllerPitchInput AxisValue))

(event Input|AxisEvents|InputAxislookright
  (params (AxisValue :type Float%20%28single-precision%29))
  (Pawn|Input|AddControllerYawInput AxisValue))

(event Input|KeyboardEvents|Z
  (params (Key :type Key%20Structure :default "None"))
  (:Pressed
    (Pawn|Input|AddMovementInput (Math|Vector|GetForwardVector (Variables|Character|GetMesh)) 1e+05 false)))

(event Input|KeyboardEvents|E
  (params (Key :type Key%20Structure :default "None"))
  (:Pressed
    (Pawn|Input|AddMovementInput (Math|Vector|GetForwardVector (Variables|Character|GetMesh)) 1e+05 false)))

(fn ConstructionScript)