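; Player-steered root that tunnels through voxel terrain until validated or its timer expires.
; Play starts timeline-driven movement and turning input, recording spline points on a looping timer.
; Each tick of that timer adds spline meshes along the whole spline without clearing earlier ones, end-scaled by a timeline.
; A forward trace carves spheres from the VoxelWorld, or notifies a hit Interactible and then destroys the root.
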(event Custom|EndRoot
  (Audio|Components|Audio|Stop (Variables|Default|GetLooping))
  (Variables|Default|SetShouldMove false)
  (CallFunction|TerminanteBranch))

(event Custom|PopulateSpline
  (if (Variables|Default|GetShouldMove)
    (Spline|AddSplinePoint (Variables|Default|GetSpline) (Transformation|GetActorLocation) "World" true))
  (CallFunction|UpdateSplineMesh))

(event Custom|UpdateSplineMesh
  (bind _returnvalue (Transformation|GetActorTransform))
  (bind _spline (Variables|Default|GetSpline))
  (bind _spacing (Variables|Default|GetSpacing))
  (bind _scaleofroot (Variables|Default|GetScaleOfRoot))
  (bind _scale (Math|Transform|BreakTransform _returnvalue))
  (bind _x (Math|Vector|BreakVector _scale))
  (bind _returnvalue_2 (* _spacing _x))
  (if (Variables|Default|GetShouldMove)
    (for _index (range 0 (.ReturnValue (Math|Float|Division(WholeandRemainder) (Spline|GetSplineLength (Variables|Default|GetSpline)) _returnvalue_2)))
      (Variables|Default|SetsplineLocation (* _returnvalue_2 _index))
      (bind _returnvalue_3 (AddComponent|AddSplineMeshComponent true))
      (Transformation|SetMobility _returnvalue_3 "Stationary")
      (Components|StaticMesh|SetStaticMesh _returnvalue_3 (Variables|Default|GetNew%20Mesh))
      (Utilities|Array|Add (Variables|Default|GetStaticMeshArray) _returnvalue_3)
      (Transformation|AttachComponentToComponent _returnvalue_3 (Variables|Default|GetSpline) "None" "KeepRelative" "KeepRelative" "KeepRelative" true)
      (SplineMesh|SetEndScale _returnvalue_3 (Math|Vector2D|MakeVector2D _scaleofroot _scaleofroot) true :!class /Script/Engine.SplineMeshComponent)
      (SplineMesh|SetStartandEnd _returnvalue_3 (Spline|GetLocationatDistanceAlongSpline _spline (Variables|Default|GetsplineLocation) "Local") (Spline|GetTangentatDistanceAlongSpline _spline (Variables|Default|GetsplineLocation) "Local") (Spline|GetLocationatDistanceAlongSpline _spline (+ (Variables|Default|GetsplineLocation) 1e+02) "Local") (Spline|GetTangentatDistanceAlongSpline _spline (+ (Variables|Default|GetsplineLocation) 1e+02) "Local") true :!class /Script/Engine.SplineMeshComponent))
    (Variables|Default|SetLastModif _index)))

(event Custom|TerminanteBranch)

(event Custom|Play
  (bind _spline (Variables|Default|GetSpline))
  (CallFunction|EnableControls)
  (CallFunction|Dig)
  (Utilities|FlowControl|Sequence
    (:then_0
      (Transformation|DetachFromComponent (Variables|Default|GetSpline) "KeepWorld" "KeepWorld" "KeepWorld" true)
      (Variables|Default|SetStartPos (Spline|GetLocationatSplinePoint _spline 0 "Local"))
      (for _index (range 1 (Spline|GetNumberOfSplinePoints _spline))
        (Spline|RemoveSplinePoint (Variables|Default|GetSpline) _index true))
      (Variables|Default|SetCurrentActorRotation (.Roll (Math|Rotator|BreakRotator (Transformation|GetActorRotation))))
      (Utilities|Time|SetTimerbyEvent (delegate Custom|EndRoot) (Variables|Default|GetTimeForRoot))
      (Utilities|Time|SetTimerbyEvent (delegate Custom|PopulateSpline) 0.25 true))
    (:then_1
      (Components|Timeline|SetPlayRate (Variables|Default|GetScaling) (/ 1.0 (Variables|Default|GetTimeForRoot)))
      (bind _newtrack_0 (Timeline|Scaling PlayFromStart)
        (:Update
          (Variables|Default|SetScaleOfRoot _newtrack_0))))))

(event Custom|EnableControls
  (Timeline|Timeline_0 Play
    (:Update
      (if (Variables|Default|GetShouldMove)
        (Transformation|SetWorldLocation (Variables|Default|GetROOT) (* (+ (Transformation|GetWorldLocation (Variables|Default|GetROOT)) (Math|Vector|GetUpVector (Transformation|GetWorldRotation (Variables|Default|GetRootEnd)))) (Variables|Default|GetMiningSpeed)) false false)))))

(event Input|ActionEvents|InputActionTurnLeft
  (params (Key :type Key%20Structure :default "None"))
  (bind _returnvalue (Transformation|GetActorRotation))
  (bind (_roll _pitch _yaw) (Math|Rotator|BreakRotator _returnvalue))
  (:Pressed
    (Timeline|RotateLeftTL Play
      (:Update
        (Variables|Default|SetCurrentActorRotation _yaw)
        (Transformation|SetActorRotation (Math|Rotator|MakeRotator _roll _pitch (+ (Variables|Default|GetCurrentActorRotation) (Variables|Default|GetTurnRate)))))))
  (:Released
    (Timeline|RotateLeftTL Stop)))

(event Input|ActionEvents|InputActionTurnRight
  (params (Key :type Key%20Structure :default "None"))
  (bind _returnvalue (Transformation|GetActorRotation))
  (bind (_roll _pitch _yaw) (Math|Rotator|BreakRotator _returnvalue))
  (:Pressed
    (Timeline|RotateRightTL Play
      (:Update
        (Variables|Default|SetCurrentActorRotation _yaw)
        (Transformation|SetActorRotation (Math|Rotator|MakeRotator _roll _pitch (- (Variables|Default|GetCurrentActorRotation) (Variables|Default|GetTurnRate)))))))
  (:Released
    (Timeline|RotateRightTL Stop)))

(event Input|ActionEvents|InputActionValidate
  (params (Key :type Key%20Structure :default "None"))
  (:Pressed
    (Audio|Components|Audio|Stop (Variables|Default|GetLooping))
    (Variables|Default|SetShouldMove false)
    (CallFunction|TerminanteBranch)))

(event Custom|Dig
  (bind _returnvalue (Transformation|GetActorLocation))
  (Timeline|TL_Dig PlayFromStart
    (:Update
      (bind (_outhit _returnvalue_2) (Collision|LineTraceByChannel _returnvalue (+ _returnvalue (* (Math|Vector|GetForwardVector (Variables|Default|GetROOT self)) (Variables|Default|GetNewVar_0))) "TraceTypeQuery1" false 0 "None"))
      (if _returnvalue_2
        (bind _returnvalue_3 (Actor|GetActorOfClass "/Script/Voxel.VoxelWorld"))
        (if (== _returnvalue_3 (.HitActor (Collision|BreakHitResult _outhit)))
          (Class|VoxelSphereTools|RemoveSphere _returnvalue_3 (.ImpactPoint (Collision|BreakHitResult _outhit)) 1e+02)
          (elif (.bSuccess (Utilities|Casting|CastToInteractible (.HitActor (Collision|BreakHitResult _outhit))))
            (Class|Interactible|OnHitComponent (.AsInteractible (Utilities|Casting|CastToInteractible (.HitActor (Collision|BreakHitResult _outhit)))) 0 0 0 "0, 0, 0" _outhit)
            (Utilities|FlowControl|Delay 0.2)
            (Actor|DestroyActor)))))))

(fn ConstructionScript)